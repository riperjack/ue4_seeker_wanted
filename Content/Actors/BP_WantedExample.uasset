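; BP_WantedExample is an example actor that shows its WantedComponent's detection state through the color of its mesh.
; On BeginPlay it creates a dynamic material instance from the mesh's first material slot.
; Every Tick it sets the MainColor parameter to green, overriding it with red when detected, or yellow when the detected actor is also flagged as closest or most distant.
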(event `self.ReceiveBeginPlay`
  (`parent.ReceiveBeginPlay`)
  (bind _returnvalue (`PrimitiveComponent.CreateDynamicMaterialInstance` (`self.MeshComponent`) 0 null "None"))
  (set `self.MainColor` _returnvalue))

(event `self.ReceiveTick`
  (params (DeltaSeconds :type "Float (single-precision)"))
  (bind _wantedcomponent (`self.WantedComponent`))
  (`MaterialInstanceDynamic.SetVectorParameterValue` (`self.MainColor`) "MainColor" (struct :`G` 1.0 :`A` 1.0))
  (if (`WantedComponent.bIsDetected` (`self.WantedComponent`))
    (`MaterialInstanceDynamic.SetVectorParameterValue` (`self.MainColor`) "MainColor" (struct :`R` 1.0 :`A` 1.0))
    (if (or (`WantedComponent.bIsClosest` _wantedcomponent) (`WantedComponent.bIsIsMostDistant` _wantedcomponent))
      (`MaterialInstanceDynamic.SetVectorParameterValue` (`self.MainColor`) "MainColor" (struct :`R` 1.0 :`G` 1.0 :`A` 1.0)))))

(fn `UserConstructionScript`
  (`parent.UserConstructionScript`))